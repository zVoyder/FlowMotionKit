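; BP_FlowMotionCharacter is a player character that can wall run and rail grind through its WallRunner and RailGrinder components.
; The attach and detach input actions are forwarded to both components at once, so one control pair drives both moves.
; Launch events from either component play a 2D jump sound through PlayEffectSound, while their attach and detach events are empty stubs.
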(event `EnhancedInput|/Game/Core/Inputs/Actions/IA_AttachToWall`
  (params (ActionValue :type Boolean) (ElapsedSeconds :type "Float (double-precision)") (TriggeredSeconds :type "Float (double-precision)") (InputAction :type "InputAction Object Reference" :default "/Game/Core/Inputs/Actions/IA_AttachToWall.IA_AttachToWall"))
  (:`Triggered`
    (`WallRunner.AttachToWall` (`self.WallRunner`))
    (`RailGrinder.AttachToRail` (`self.RailGrinder`))))

(event `EnhancedInput|/Game/Core/Inputs/Actions/IA_DetachFromWall`
  (params (ActionValue :type Boolean) (ElapsedSeconds :type "Float (double-precision)") (TriggeredSeconds :type "Float (double-precision)") (InputAction :type "InputAction Object Reference" :default "/Game/Core/Inputs/Actions/IA_DetachFromWall.IA_DetachFromWall"))
  (:`Triggered`
    (`WallRunner.DetachFromWall` (`self.WallRunner`))
    (`RailGrinder.DetachFromRail` (`self.RailGrinder`))))

(event `self.WallRunner.OnWallRunAttach`
  ;[1 0 0 0.5] Wall Run Events
)

(event `self.WallRunner.OnWallRunDetach`
  ;[1 0 0 0.5] Wall Run Events
)

(event `self.WallRunner.OnWallRunLaunch`
  ;[1 0 0 0.5] Wall Run Events
  (`self.PlayEffectSound`))

(event `self.RailGrinder.OnRailGrindAttach`
  ;[1 0 0 0.5] Rail Grind Events
)

(event `self.RailGrinder.OnRailGrindDetach`
  ;[1 0 0 0.5] Rail Grind Events
)

(event `self.RailGrinder.OnRailGrindLaunch`
  ;[1 0 0 0.5] Rail Grind Events
  (`self.PlayEffectSound`))

(fn `UserConstructionScript`)