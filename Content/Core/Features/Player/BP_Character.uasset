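; Player character Blueprint that forwards wall-running input to a WallRunner component.
; Enhanced Input actions for attaching to and detaching from walls call the matching functions on that component.
; A debug Q key release sets the movement component's gravity scale.
; Launch, disable-movement and disable-input nodes are present but disconnected, and BeginPlay, Tick and the construction script are empty.
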(event Input|EnhancedActionEvents|EnhancedInputActionIA_AttachToWall
  (params (ActionValue :type Boolean) (ElapsedSeconds :type Float%20%28double-precision%29) (TriggeredSeconds :type Float%20%28double-precision%29) (InputAction :type Input%20Action%20Object%20Reference :default "/Game/Core/Inputs/Actions/IA_AttachToWall.IA_AttachToWall"))
  (Class|WallRunner|AttachtoWall (Variables|Default|GetWallRunner)))

(event Input|EnhancedActionEvents|EnhancedInputActionIA_DetachFromWall
  (params (ActionValue :type Boolean) (ElapsedSeconds :type Float%20%28double-precision%29) (TriggeredSeconds :type Float%20%28double-precision%29) (InputAction :type Input%20Action%20Object%20Reference :default "/Game/Core/Inputs/Actions/IA_DetachFromWall.IA_DetachFromWall"))
  (Class|WallRunner|DetachfromWall (Variables|Default|GetWallRunner)))

(event EventTick
  (params (DeltaSeconds :type Float%20%28single-precision%29)))

(event EventBeginPlay)

(event Input|KeyboardEvents|DebugKeyQ
  (params (Key :type Key%20Structure :default "None") (ActionValue :type Input%20Action%20Value%20Structure))
  (:Released
    (Variables|/Script/Engine.CharacterMovementComponent|SetGravityScale (Variables|Character|GetCharacterMovement) 1.75)))

(fn ConstructionScript)